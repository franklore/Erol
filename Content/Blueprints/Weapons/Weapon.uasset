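; Base weapon actor that handles trigger input, pickup and drop, leaving Fire and the fire/reload animations as empty stubs.
; FireDown either starts a looping Fire timer for automatic weapons, stopped by FireUp, or fires once and re-enables via ResetGun after the fire interval.
; The WeaponOwner RepNotify drives Pickup, which disables physics and collision and notifies the owner, or Drop, which detaches, restores them and delays re-pickup.
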(event `DelayEnablePickUp`
  (`KismetSystemLibrary.Delay` 2.0)
  (set `self.EnablePickUp` true))

(fn `Drop`
  (bind _weaponmesh (`self.WeaponMesh`))
  (`self.DelayEnablePickUp`)
  (`self.SetActorEnableCollision` true)
  (`PrimitiveComponent.SetSimulatePhysics` _weaponmesh true)
  (`self.K2_DetachFromActor` "KeepRelative")
  (`SceneComponent.SetVisibility` _weaponmesh true false)
  (`self.FireUp`))

(fn `Fire`)

(fn `FireDown`
  (if (`self.EnableFiring`)
    (if (`self.AutoFire`)
      (`self.Fire`)
      (bind _returnvalue (`KismetSystemLibrary.K2_SetTimer` null "Fire" (`self.FireInterval`) true))
      (set `self.AutoFireTimerHandle` _returnvalue)
      (elif (`self.EnableFiring`)
        (set `self.EnableFiring` false)
        (`self.Fire`)
        (`KismetSystemLibrary.K2_SetTimer` null "ResetGun" (`self.FireInterval`))))))

(fn `FireUp`
  (if (`self.AutoFire`)
    (`KismetSystemLibrary.K2_ClearAndInvalidateTimerHandle` (`self.AutoFireTimerHandle`))))

(fn `OnRep_WeaponOwner`
  (`/Engine/EditorBlueprintResources/StandardMacros.IsValid` (`self.WeaponOwner`)
    (:`Is Valid`
      (`self.Pickup`))
    (:`Is Not Valid`
      (`self.Drop`))))

(fn `Pickup`
  (bind _weaponowner (`self.WeaponOwner`))
  (`self.SetActorEnableCollision` false)
  (`PrimitiveComponent.SetSimulatePhysics` (`self.WeaponMesh`) false)
  (`self.SetOwner` _weaponowner)
  (message `/Game/Blueprints/Weapons/WeaponUser.Equip` _weaponowner self)
  (set `self.EnablePickUp` false))

(fn `PlayFireAnim`)

(fn `PlayReloadAnim`)

(fn `ResetGun`
  (set `self.EnableFiring` true))

(fn `UserConstructionScript`)