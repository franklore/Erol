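; Ray gun weapon that fires a hitscan line trace from the muzzle socket, ignoring its owner.
; Fire plays effects locally, sends damage to DamageTaker actors and calls SubmitFire, which sends damage again with doubled headshots.
; SubmitFire also calls MulticastFireEffect, replaying effects on simulated proxies.
; SpawnFX plays the fire animation and picks impact sound and particles by character, head or physical surface; its tracer code is unconnected.
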(event `Submit Fire`
  (params (hit :type "HitResult Structure"))
  (bind (_bblockinghit _binitialoverlap _time _distance _location _impactpoint _normal _impactnormal _physmat _hitactor _hitcomponent _hitbonename) (`GameplayStatics.BreakHitResult` hit))
  (bind _damage (`self.Damage`))
  (bind _returnvalue (== _hitbonename "head"))
  (`self.Multicast FireEffect` hit)
  (if (`KismetSystemLibrary.DoesImplementInterface` _hitactor "/Game/Blueprints/Weapons/Damagetaker.DamageTaker_C")
    (message `/Game/Blueprints/Weapons/Damagetaker.TakeDamage` _hitactor (make `/Game/Blueprints/Weapons/Damage` (select `bool` _returnvalue :`false` _damage :`true` (* _damage 2.0)) (select `bool` _returnvalue :`false` "NewEnumerator0" :`true` "NewEnumerator1" :!type "/Game/Blueprints/Weapons/DamageType Enum") (`self.WeaponOwner`)))))

(event `Multicast FireEffect`
  (params (hit :type "HitResult Structure"))
  (if (`|EnumEquality` (`self.GetLocalRole` (`self.GetOwner`)) "ROLE_SimulatedProxy")
    (`self.PlayFireEffect` hit)))

(fn `Fire`
  (bind _weaponowner (`self.WeaponOwner`))
  (bind (_returnvalue_location _returnvalue_rotation) (`KismetMathLibrary.BreakTransform` (`SceneComponent.GetSocketTransform` (`self.WeaponMesh`) "MuzzleFlash" "RTS_World")))
  (`/Engine/EditorBlueprintResources/StandardMacros.IsValid` _weaponowner
    (:`Is Valid`
      (bind _outhit (`KismetSystemLibrary.LineTraceSingle` _returnvalue_location (+ _returnvalue_location (* (`KismetMathLibrary.GetForwardVector` _returnvalue_rotation) (`self.ShootRange`))) "TraceTypeQuery3" false (`|MakeArray` _weaponowner :!type "Actor Object Reference")))
      (`self.Submit Fire` _outhit)
      (`self.PlayFireEffect` _outhit)
      (bind (_bblockinghit _binitialoverlap _time _distance _location _impactpoint _normal _impactnormal _physmat _hitactor _hitcomponent _hitbonename) (`GameplayStatics.BreakHitResult` _outhit))
      (if (`KismetSystemLibrary.DoesImplementInterface` _hitactor "/Game/Blueprints/Weapons/Damagetaker.DamageTaker_C")
        (message `/Game/Blueprints/Weapons/Damagetaker.TakeDamage` _hitactor (make `/Game/Blueprints/Weapons/Damage` (`self.Damage`) (select `bool` (== _hitbonename "head") :`false` "NewEnumerator0" :`true` "NewEnumerator1" :!type "/Game/Blueprints/Weapons/DamageType Enum") _weaponowner))))))

(fn `PlayFireEffect`
  (params (hit :type "HitResult Structure"))
  (`self.SpawnFX` hit)
  (`self.OnFired`))

(fn `SpawnFX`
  (params (Hit :type "HitResult Structure"))
  (bind (_bblockinghit _binitialoverlap _time _distance _location _impactpoint _normal _impactnormal _physmat _hitactor _hitcomponent _hitbonename) (`GameplayStatics.BreakHitResult` Hit))
  (`|ExecutionSequence`
    (:`then_0`
      (`self.PlayFireAnim`))
    (:`then_2`
      ;[1 1 1] hit
      (if _bblockinghit
        (cast `Character` _hitactor
          (:`then`
            (set `self.HitCharacter` true))
          (:`CastFailed`
            (set `self.HitCharacter` false)))
        (if (== _hitbonename "head")
          (set `self.HitHead` true)
          (else
            (set `self.HitHead` false)))
        (`GameplayStatics.SpawnSoundAtLocation` (select `bool` (`self.HitCharacter`) :`false` (`self.HitCharacterSound`) :`true` (`self.HitSurfaceSound`)) _location (struct) 1.0 1.0 0.0 null null)
        (`GameplayStatics.SpawnEmitterAtLocation` (select `bool` (`self.HitCharacter`) :`false` (select `EPhysicalSurface` (`PhysicalMaterial.SurfaceType` _physmat) :`SurfaceType_Default` (`self.HitDefaultEmitter`) :`SurfaceType1` (`self.HitStoneEmitter`) :`SurfaceType2` (`self.HitMetalEmitter`) :`SurfaceType3` (`self.HitWoodEmitter`)) :`true` (select `bool` (`self.HitHead`) :`false` (`self.HitCharacterEmitter`) :`true` (`self.HitCharacterHeadEmitter`))) _location)))))

(fn `UserConstructionScript`
  (`parent.UserConstructionScript`))