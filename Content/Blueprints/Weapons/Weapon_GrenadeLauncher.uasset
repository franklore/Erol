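; Grenade launcher weapon Blueprint, extending a parent weapon class, that launches physical grenade projectiles from its muzzle socket.
; Fire passes the muzzle transform to SubmitFire and plays the animation and fired callback locally.
; SubmitFire spawns a grenade, makes it and the owner's collision component ignore each other when moving, and applies a forward impulse.
; MulticastFireEffect repeats the effect only where the owner is a simulated proxy, avoiding double playback for the shooter.
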(event `Submit Fire`
  (params (FireTransform :type "Transform Structure"))
  (`self.Spawn Ammo`)
  (`self.Multicast FireEffect`))

(event `Spawn Ammo`
  (bind _weaponowner (`self.WeaponOwner`))
  (bind _returnvalue (`|SpawnActorFromClass` "/Game/Blueprints/Weapons/Grenade_Ammo.Grenade_Ammo_C" (stale `Submit Fire` FireTransform) "Undefined" "OverrideRootScale" _weaponowner _weaponowner))
  (bind _collisioncomponent (message `/Game/Blueprints/Weapons/WeaponUser.GetCollisionComponent` _weaponowner))
  (bind _staticmesh (`/Game/Blueprints/Weapons/Grenade_Ammo.StaticMesh` _returnvalue))
  (`PrimitiveComponent.IgnoreComponentWhenMoving` _staticmesh _collisioncomponent true)
  (`PrimitiveComponent.IgnoreComponentWhenMoving` _collisioncomponent _staticmesh true)
  (`PrimitiveComponent.AddImpulse` _staticmesh (* (`KismetMathLibrary.GetForwardVector` (.rotation (stale `Submit Fire` FireTransform))) 800.0) "None" false))

(event `Multicast FireEffect`
  (if (`|EnumEquality` (`self.GetLocalRole` (`self.GetOwner`)) "ROLE_SimulatedProxy")
    (`self.FireEffect`)))

(fn `Fire`
  (`self.Submit Fire` (`SceneComponent.GetSocketTransform` (`self.WeaponMesh`) "MuzzleFlash" "RTS_World"))
  (`self.FireEffect`))

(fn `FireDown`
  (`parent.FireDown`))

(fn `FireEffect`
  (`self.PlayFireAnim`)
  (`self.OnFired`))

(fn `FireUp`
  (`parent.FireUp`))

(fn `PlayFireAnim`
  (`SkeletalMeshComponent.PlayAnimation` (`self.WeaponMesh`) "/Game/MilitaryWeapDark/Weapons/Anims/Fire_GrenadeLauncher_W.Fire_GrenadeLauncher_W" false))

(fn `UserConstructionScript`
  (`parent.UserConstructionScript`))