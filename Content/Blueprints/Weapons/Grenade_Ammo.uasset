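; Grenade projectile actor that explodes on hitting a Character and plays a multicast bounce sound on other hard impacts.
; BeginPlay also starts a two-second timer, though its bound event is not shown.
; Explode spawns particles and sound on the Remote branch only, applies radial impulse to meshes of overlapped non-Pawn actors, then destroys itself.
; Distance-scaled DamageTaker damage is disconnected, and the surface-type switch does nothing.
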(event `self.ReceiveHit`
  (params (MyComp :type "PrimitiveComponent Object Reference") (Other :type "Actor Object Reference") (OtherComp :type "PrimitiveComponent Object Reference") (bSelfMoved :type Boolean) (HitLocation :type "Vector Structure") (HitNormal :type "Vector Structure") (NormalImpulse :type "Vector Structure") (Hit :type "HitResult Structure (by ref)"))
  (cast `Character` Other
    (:`then`
      (`self.Explode`))
    (:`CastFailed`
      (if (> (`KismetMathLibrary.VSize` NormalImpulse) 1000.0)
        (switch `EPhysicalSurface` (`PhysicalMaterial.SurfaceType` (`.PhysMat` (`GameplayStatics.BreakHitResult` Hit)))
          (:`SurfaceType_Default`
            _)
          (:`SurfaceType1`
            _)
          (:`SurfaceType2`
            _)
          (:`SurfaceType3`
            _))
        (`self.Multicast HitSound`)))))

(event `self.ReceiveBeginPlay`
  (`KismetSystemLibrary.K2_SetTimerDelegate` (`|CreateDelegate` :!event `Explode`) 2.0))

(event `Explode`
  (bind _returnvalue (`self.K2_GetActorLocation`))
  (`|ExecutionSequence`
    (:`then_0`
      (`/Engine/EditorBlueprintResources/ActorMacros.Switch Has Authority`
        (:`Remote`
          (`GameplayStatics.SpawnEmitterAtLocation` "/Game/MilitaryWeapDark/FX/P_Grenade_Explosion_01.P_Grenade_Explosion_01" _returnvalue)
          (`GameplayStatics.PlaySoundAtLocation` "/Game/MilitaryWeapDark/Sound/GrenadeLauncher/GrenadeLauncher_Explosion_Cue.GrenadeLauncher_Explosion_Cue" _returnvalue (struct) 1.0 1.0 0.0 null null null))))
    (:`then_1`
      (bind _outactors (`KismetSystemLibrary.SphereOverlapActors` _returnvalue (`self.ExplodeRadius`) (`|MakeArray` "ObjectTypeQuery2" "ObjectTypeQuery3" :!type "EObjectTypeQuery Enum")))
      (for _array_element _outactors
        (bind _aspawn (cast `Pawn` _array_element)
          (:`then`
            (if (`KismetSystemLibrary.DoesImplementInterface` _aspawn "/Game/Blueprints/Weapons/Damagetaker.DamageTaker_C")
              _))
          (:`CastFailed`
            (bind _returnvalue_2 (`self.GetComponentByClass` _array_element "/Script/Engine.MeshComponent"))
            (if (`KismetSystemLibrary.IsValid` _returnvalue_2)
              (`PrimitiveComponent.AddRadialImpulse` _returnvalue_2 _returnvalue (`self.ExplodeRadius`) 100000.0 "RIF_Constant" false))))))
    (:`then_2`
      (`self.K2_DestroyActor`))))

(event `Multicast HitSound`
  (`GameplayStatics.PlaySoundAtLocation` "/Game/MilitaryWeapDark/Sound/GrenadeLauncher/GrenadeLauncher_Lower_Cue.GrenadeLauncher_Lower_Cue" (`self.K2_GetActorLocation`) (struct) 1.0 1.0 0.0 null null null))

(fn `UserConstructionScript`)