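; BP_Target is a scoring target actor that rates a location from 0 to 10 by its closeness to the target's origin.
; GetScore drops the score in floored distance steps, scaled by the actor's X scale so larger targets have wider bands.
; BeginPlay normalizes Direction and starts a looping timer that reverses it every Duration seconds.
; The movement step along Direction at Speed is disconnected from the empty Tick, so the target does not move itself.
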(event `self.ReceiveBeginPlay`
  (`KismetSystemLibrary.K2_SetTimer` null "ChangeDirection" (`self.duration`) true)
  (set `self.Direction` (`KismetMathLibrary.Normal` (`self.Direction`))))

(event `self.ReceiveTick`
  (params (DeltaSeconds :type "Float (single-precision)")))

(fn `ChangeDirection`
  (set `self.Direction` (`KismetMathLibrary.NegateVector` (`self.Direction`))))

(fn `GetScore`
  (params (Location :type "Vector Structure"))
  (returns (score :type Integer))
  (bind _returnvalue (`self.GetTransform`))
  (return (`KismetMathLibrary.Clamp` (- 10 (`KismetMathLibrary.FFloor` (/ (* (`KismetMathLibrary.Vector_Distance` Location (.location _returnvalue)) 0.2) (.x (.scale _returnvalue))))) 0 10)))

(fn `UserConstructionScript`)