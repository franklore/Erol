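; Player controller that builds the local player's UI and handles match start and end feedback.
; After login it creates the HUD, a hidden pause menu and a screen text widget, only on the local controller.
; It forwards ready signals to the game mode and shows a countdown when the mission is ready.
; At mission end it shows win or lose from the game state, adding a record widget for winners with a nonzero rank.
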(event `ClientPostLogin`
  (`self.DrawHUD`))

(event `SendReadySIgnal`
  (bind _asbp_erol_game_mode (cast `/Game/Blueprints/BP_ErolGameMode` (`GameplayStatics.GetGameMode`)))
  (`/Game/Blueprints/BP_ErolGameMode.Ready` _asbp_erol_game_mode self))

(event `MissionReady`
  (bind _screeninfotext (`self.ScreenInfoText`))
  (`/Game/HUD/ScreenInfoText.ShowInfoText1s` _screeninfotext "3")
  (`KismetSystemLibrary.Delay` 1.0)
  (`/Game/HUD/ScreenInfoText.ShowInfoText1s` _screeninfotext "2")
  (`KismetSystemLibrary.Delay` 1.0)
  (`/Game/HUD/ScreenInfoText.ShowInfoText1s` _screeninfotext "1")
  (`KismetSystemLibrary.Delay` 1.0)
  (`/Game/HUD/ScreenInfoText.ShowInfoText1s` _screeninfotext "Go!"))

(event `MissionEnd`
  (bind _screeninfotext (`self.ScreenInfoText`))
  (bind _asbp_erol_game_state (cast `/Game/Blueprints/BP_ErolGameState` (`GameplayStatics.GetGameState`)))
  (bind _asbp_erol_player_state (cast `/Game/Blueprints/BP_ErolPlayerState` (`self.PlayerState`)))
  (if (== (`/Game/Blueprints/BP_ErolPlayerState.PlayerNumber` _asbp_erol_player_state) (`/Game/Blueprints/BP_ErolGameState.WinnerID` _asbp_erol_game_state))
    (`/Game/HUD/ScreenInfoText.ShowInfoText1s` _screeninfotext "Win!")
    (bind _rank (`/Game/Blueprints/BP_ErolGameState.GetRank` _asbp_erol_game_state (`/Game/Blueprints/BP_ErolGameState.WinnerScore` _asbp_erol_game_state)))
    (if (!= _rank 0)
      (bind _returnvalue (`|CreateWidget` "/Game/HUD/BreakRecord.BreakRecord_C"))
      (bind _output_get (set `self.BreakRecordWidget` _returnvalue))
      (`UserWidget.AddToViewport` _output_get 0))
    (else
      (`/Game/HUD/ScreenInfoText.ShowInfoText1s` _screeninfotext "Lose!"))))

(fn `DrawHUD`
  (if (`self.IsLocalPlayerController`)
    (`|ExecutionSequence`
      (:`then_0`
        (bind _returnvalue (`|CreateWidget` "/Game/HUD/ErolHUD.ErolHUD_C" self))
        (bind _output_get (set `self.HUD` _returnvalue))
        (`UserWidget.AddToViewport` _output_get 0))
      (:`then_1`
        (bind _returnvalue_2 (`|CreateWidget` "/Game/HUD/PauseMenu.PauseMenu_C" self))
        (bind _output_get_2 (set `self.PauseMenu` _returnvalue_2))
        (`Widget.SetVisibility` _output_get_2 "Hidden")
        (`UserWidget.AddToViewport` _output_get_2 0))
      (:`then_2`
        (bind _returnvalue_3 (`|CreateWidget` "/Game/HUD/ScreenInfoText.ScreenInfoText_C"))
        (bind _output_get_3 (set `self.ScreenInfoText` _returnvalue_3))
        (`UserWidget.AddToViewport` _output_get_3 0)))))

(fn `UserConstructionScript`)