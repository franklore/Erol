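; BP_ErolGameState is a game state that relays mission flow events and keeps a score leaderboard.
; MissionReady and MissionEnd forward to the first player's BP_PlayerController.
; SubmitRank inserts a record above the first lower score in Ranks, then drops the last entry if the list exceeds RankSize.
; A record that beats no existing entry is not added, so an empty list stays empty.
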(event `MissionReady`
  (bind _asbp_player_controller (cast `/Game/Blueprints/BP_PlayerController` (`GameplayStatics.GetPlayerController` 0)))
  (`/Game/Blueprints/BP_PlayerController.MissionReady` _asbp_player_controller))

(event `MissionEnd`
  (bind _asbp_player_controller (cast `/Game/Blueprints/BP_PlayerController` (`GameplayStatics.GetPlayerController` 0)))
  (`/Game/Blueprints/BP_PlayerController.MissionEnd` _asbp_player_controller))

(event `SubmitRank`
  (params (Rank :type "/Game/HUD/RankRecord Structure"))
  (`self.Insert Rank` Rank))

(fn `GetRank`
  (params (Score :type Integer))
  (returns (Rank :type Integer))
  (for (_array_element _array_index) (`self.Ranks`)
    (if (> Score (`.Score_5_C6CF01B14E991FF4A31F8CB161F0C82E` (break `/Game/HUD/RankRecord` _array_element)))
      (return (+ _array_index 1))))
  (return 0))

(fn `Insert Rank`
  (params (Record :type "/Game/HUD/RankRecord Structure"))
  (bind _ranks (`self.Ranks`))
  (bind _rank (`self.GetRank` (`.Score_5_C6CF01B14E991FF4A31F8CB161F0C82E` (break `/Game/HUD/RankRecord` Record))))
  (if (> _rank 0)
    (`KismetArrayLibrary.Array_Insert` _ranks Record (- _rank 1))
    (if (> (`KismetArrayLibrary.Array_Length` (`self.Ranks`)) (`self.RankSize`))
      (`KismetArrayLibrary.Array_Remove` _ranks (`KismetArrayLibrary.Array_LastIndex` _ranks)))))

(fn `UserConstructionScript`)