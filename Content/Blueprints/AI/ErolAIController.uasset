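; AI controller for computer players that gives each one a player number and an "AI" name, then runs a randomly chosen crazy or patrol behavior tree on possess.
; Perception updates set the enemy and shoot flag in the blackboard, with a short timer delaying their clearing after sight is lost.
; Health updates are mirrored to the blackboard, and a kill of the current enemy turns off shooting.
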(event `self.ReceiveBeginPlay`
  (bind _asbp_erol_player_state (cast `/Game/Blueprints/BP_ErolPlayerState` (`self.PlayerState`)))
  (bind _asbp_erol_game_mode (cast `/Game/Blueprints/BP_ErolGameMode` (`GameplayStatics.GetGameMode`)))
  (bind _newparam (`/Game/Blueprints/BP_ErolGameMode.GetPlayerNumber` _asbp_erol_game_mode))
  (set `/Game/Blueprints/BP_ErolPlayerState.PlayerNumber` _newparam _asbp_erol_player_state)
  (set `/Game/Blueprints/BP_ErolPlayerState.playerName` (`KismetTextLibrary.Conv_StringToText` (`KismetStringLibrary.Concat_StrStr` "AI" (`KismetStringLibrary.Conv_IntToString` (`/Game/Blueprints/BP_ErolPlayerState.PlayerNumber` _asbp_erol_player_state)))) _asbp_erol_player_state))

(event `self.AIPerception.OnTargetPerceptionUpdated`
  (params (Actor :type "Actor Object Reference") (Stimulus :type "AIStimulus Structure"))
  (bind _blackboard (`self.Blackboard`))
  (if (`.bSuccessfullySensed` (break `AIStimulus` Stimulus))
    (`KismetSystemLibrary.K2_ClearAndInvalidateTimerHandle` (`self.EnemyTimer`))
    (`BlackboardComponent.SetValueAsBool` _blackboard (`self.CanShootEnemy`) true)
    (`BlackboardComponent.SetValueAsObject` _blackboard (`self.EnemyActor`) Actor)
    (else
      (bind _returnvalue (`KismetSystemLibrary.K2_SetTimerDelegate` (delegate `StartEnemyTimer`) 1.0))
      (set `self.EnemyTimer` _returnvalue))))

(event `StartEnemyTimer`
  (bind _blackboard (`self.Blackboard`))
  (`BlackboardComponent.SetValueAsBool` _blackboard (`self.CanShootEnemy`) false)
  (`BlackboardComponent.SetValueAsObject` _blackboard (`self.EnemyActor`) null))

(event `On Killed`
  (params (character :type "Character Object Reference"))
  (bind _blackboard (`self.Blackboard`))
  (if (== character (`BlackboardComponent.GetValueAsObject` _blackboard (`self.EnemyActor`)))
    (`BlackboardComponent.SetValueAsBool` _blackboard (`self.CanShootEnemy`) false)))

(event `OnUpdateHealth`
  (params (Health :type "Float (double-precision)"))
  (`BlackboardComponent.SetValueAsFloat` (`self.Blackboard`) (`self.SelfHealth`) Health))

(event `self.ReceivePossess`
  (params (PossessedPawn :type "Pawn Object Reference"))
  (`self.RunBehaviorTree` (select `int` (`KismetMathLibrary.RandomInteger` 2) :`0` "/Game/Blueprints/AI/BT_CrazyAI.BT_CrazyAI" :`1` "/Game/Blueprints/AI/BT_PatrolAI.BT_PatrolAI" :!type "BehaviorTree Object Reference")))

(fn `UserConstructionScript`)