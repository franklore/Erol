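; Game instance Blueprint that opens the main menu and manages LAN multiplayer sessions.
; ShowMainMenu adds the menu widget on anything but a dedicated server.
; HostServer creates a two-connection session and opens MainMap as a listen server, while JoinServer joins the first session found; both ignore their Name input.
; QuitServer destroys the session and returns to EntryMap.
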(event `ShowMainMenu`
  (if (not (`KismetSystemLibrary.IsDedicatedServer`))
    (bind _returnvalue (`|CreateWidget` "/Game/HUD/Mainmenu.Mainmenu_C" (`GameplayStatics.GetPlayerController` 0)))
    (`UserWidget.AddToViewport` _returnvalue 0)))

(event `HostServer`
  (params (Name :type Text))
  (`CreateSessionCallbackProxy.CreateSession` (`GameplayStatics.GetPlayerController` 0) 2 true
    (:`OnSuccess`
      (`GameplayStatics.OpenLevel` "MainMap" true "listen"))))

(event `JoinServer`
  (params (Name :type Text))
  (bind _results (`FindSessionsCallbackProxy.FindSessions` (`GameplayStatics.GetPlayerController` 0) 1 true)
    (:`OnSuccess`
      (if (> (`KismetArrayLibrary.Array_Length` _results) 0)
        (`JoinSessionCallbackProxy.JoinSession` (`GameplayStatics.GetPlayerController` 0) (`|GetArrayItem` _results)
          (:`OnSuccess`
            (`KismetSystemLibrary.PrintString` "success"))
          (:`OnFailure`
            (`KismetSystemLibrary.PrintString` "fail")))))
    (:`OnFailure`
      (`KismetSystemLibrary.PrintString` "no server"))))

(event `QuitServer`
  (`DestroySessionCallbackProxy.DestroySession` (`GameplayStatics.GetPlayerController` 0)
    (:`OnSuccess`
      (`GameplayStatics.OpenLevel` "EntryMap"))))